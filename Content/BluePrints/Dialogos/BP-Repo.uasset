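; BP-Repo is a dialogue Blueprint that shows lines of conversation in an on-screen box.
; Each Hablar event increments Conversacion and writes that entry of the Dialogo array to the widget's text.
; The BPMarcoConversacion widget is created and added to the viewport only when no valid instance exists.
; Once the index passes the last line, the widget is removed, and the index is never reset here.
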(event `/Game/BluePrints/Dialogos/BP-Dialogos.hablar`
  (`/Engine/EditorBlueprintResources/StandardMacros.IncrementInt` (`self.Conversacion`)
    (:`  `
      (if (< (`self.Conversacion`) (`KismetArrayLibrary.Array_Length` (`self.Dialogo `)))
        (`self.Interfaz usuario`
          (:`then`
            _)
          (:`else`
            (bind _returnvalue (`|CreateWidget` "/Game/BluePrints/Dialogos/BP-MarcoConversacion.BP-MarcoConversacion_C" (`GameplayStatics.GetPlayerController` 0)))
            (bind _output_get (set `self.Interfaz usuario` _returnvalue))
            (`UserWidget.AddToViewport` (`self.Interfaz usuario`) 0)
            (`UserWidget.AddToViewport` _output_get 0)))
        (`TextBlock.SetText` (`/Game/BluePrints/Dialogos/BP-MarcoConversacion.Textoconversacion` (`self.Interfaz usuario`)) (`KismetTextLibrary.Conv_StringToText` (`|GetArrayItem` (`self.Dialogo `) (`self.Conversacion`))))
        (else
          (`Widget.RemoveFromParent` (`self.Interfaz usuario`)))))))

(fn `UserConstructionScript`)