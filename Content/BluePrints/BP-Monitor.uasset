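; BP-Monitor is an interactable monitor that the player switches on and off with the E key.
; A Box overlap enables input from player controller 0 and end overlap disables it, with no check on which actor overlaps.
; Each press flips Encendido and swaps material slot 1 on MeshMonitor between Lambert2SG (on) and Pantallanegra (off), which is also set at BeginPlay.
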(event `self.Box.OnComponentBeginOverlap`
  (params (OverlappedComponent :type "PrimitiveComponent Object Reference") (OtherActor :type "Actor Object Reference") (OtherComp :type "PrimitiveComponent Object Reference") (OtherBodyIndex :type Integer) (bFromSweep :type Boolean) (SweepResult :type "HitResult Structure (by ref)"))
  (`KismetSystemLibrary.PrintString` "dentro del box")
  (`self.EnableInput` (`GameplayStatics.GetPlayerController` 0)))

(event `self.ReceiveBeginPlay`
  (`PrimitiveComponent.SetMaterial` (`self.Mesh Monitor`) 1 "/Game/Pantallanegra.Pantallanegra"))

(event `self.Box.OnComponentEndOverlap`
  (params (OverlappedComponent :type "PrimitiveComponent Object Reference") (OtherActor :type "Actor Object Reference") (OtherComp :type "PrimitiveComponent Object Reference") (OtherBodyIndex :type Integer))
  (`self.DisableInput` (`GameplayStatics.GetPlayerController` 0)))

(event `Key|E`
  (params (Key :type "Key Structure"))
  (:`Pressed`
    (bind _output_get (set `self.Encendido` (not (`self.Encendido`))))
    (if _output_get
      (`PrimitiveComponent.SetMaterial` (`self.Mesh Monitor`) 1 "/Game/Computadora3/scene/Materials/lambert2SG.lambert2SG")
      (`KismetSystemLibrary.PrintString` "listo")
      (else
        (`PrimitiveComponent.SetMaterial` (`self.Mesh Monitor`) 1 "/Game/Pantallanegra.Pantallanegra")))))

(fn `UserConstructionScript`)